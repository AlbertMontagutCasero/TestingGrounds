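; Game mode for an infinite terrain game that chains BP_Tile actors at start and keeps a score of conquered tiles.
; On BeginPlay it fills a NavMeshBoundsVolume pool, then calls SpawnTile in a short loop, clearing IsFirstTile after the first pass.
; When IsFirstTile is false, SpawnTile spawns a tile, hands it the shared pool and takes its attach location as the next spawn transform.
; NewTileConquered increments Score.
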(event EventBeginPlay
  (Class|InfiniteTerrainGameMode|PopulateBoundsVolumePool)
  (for _index (range 0 4)
    (if (== _index 1)
      (Variables|Default|SetIsFirstTile false))
    (CallFunction|SpawnTile)))

(event EventTick
  (params (DeltaSeconds :type Float%20%28single-precision%29)))

(fn ConstructionScript)

(fn SpawnTile
  (if (Variables|Default|GetIsFirstTile)
    (Development|PrintString "true")
    (else
      (Development|PrintString "false")
      (bind _returnvalue (Game|SpawnActorfromClass "/Game/Dynamic/Terrain/BP_Tile.BP_Tile_C" (Variables|Default|GetNextTileTransform) "Undefined" 0 0))
      (Class|Tile|SetPool _returnvalue (Variables|Default|GetNavMeshBoundsVolumePool))
      (bind _attach_transform (Default|GetAttachLocation _returnvalue))
      (Variables|Default|SetNextTileTransform _attach_transform))))

(fn NewTileConquered
  (Math|Integer|IncrementInt (Variables|Default|GetScore)))